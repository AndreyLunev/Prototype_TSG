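; BP_NPC_Oldman is a prototype old man NPC that hands its dialogue to the player character when touched.
; On actor overlap with a BP_Character, it registers itself as that character's Something reference, copies its Dialog0 into the character and sets the character's Obj value to 2.
; It has no other active logic, so any use of that data is left to the character.
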(event `self.ReceiveActorBeginOverlap`
  (params (OtherActor :type "Actor Object Reference"))
  (bind _asbp_character (cast `/Game/Prototype/Prot_ver2/BP_Character` OtherActor))
  (set `/Game/Prototype/Prot_ver2/BP_Character.Something` self _asbp_character)
  (set `/Game/Prototype/Prot_ver2/BP_Character.Dialog0` (`self.Dialog0`) _asbp_character)
  (set `/Game/Prototype/Prot_ver2/BP_Character.Obj` 2 _asbp_character))

(fn `UserConstructionScript`
  (`parent.UserConstructionScript`))