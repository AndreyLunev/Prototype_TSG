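; Prototype player character that drives NPC dialog, object searching and a glasses quest through overlaps.
; BeginPlay creates the dialog widget; after a short delay, overlaps switch on Obj (child, old man, standard NPC, searchable, door) to load dialog and pass glasses flags to NPCs.
; End overlap collapses and clears the dialog, resetting interrupted searches.
; Tick advances QuestStatus once glasses are obtained, and held input sets a camera-lock flag.
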(event `self.ReceiveBeginPlay`
  (`parent.ReceiveBeginPlay`)
  (bind _returnvalue (`|CreateWidget` "/Game/Prototype/Prot_ver2/W_Dialog.W_Dialog_C"))
  (bind _output_get (set `self.Widget Dialog` _returnvalue))
  (`UserWidget.AddToViewport` _output_get 0)
  (set `/Game/Prototype/Prot_ver2/W_Dialog.Character` self _output_get)
  (set `/Game/Prototype/Prot_ver2/W_UI.Character` self (`self.Widget UI`))
  (set `self.QuestStatus` 0))

(event `self.ReceiveTick`
  (params (DeltaSeconds :type "Float (single-precision)"))
  (`parent.ReceiveTick` DeltaSeconds)
  (if (`self.Glases?`)
    (`/Engine/EditorBlueprintResources/StandardMacros.DoOnce` false
      (:`Completed`
        (set `self.QuestStatus` 2)))))

(event `InputAction|CameraLock`
  (params (Key :type "Key Structure"))
  (:`Pressed`
    (if (not (`self.IsLockCamera?`))
      (set `self.IsLockCamera?` true)))
  (:`Released`
    (set `self.IsLockCamera?` false)))

(event `self.ReceiveActorBeginOverlap`
  (params (OtherActor :type "Actor Object Reference"))
  (bind _widget_dialog (`self.Widget Dialog`))
  (set `self.Lockal_Something` OtherActor)
  (`KismetSystemLibrary.Delay` 0.1)
  (switch `int` (`self.Obj`)
    (:`1`
      (bind _output_get (set `/Game/Prototype/Prot_ver2/W_Dialog.DialogChar` (`self.DialogChild`) (`self.Widget Dialog`)))
      (set `TextBlock.Text` (`|GetArrayItem` _output_get) (`/Game/Prototype/Prot_ver2/W_Dialog.1-st` (`self.Widget Dialog`)))
      (set `TextBlock.Text` (`|GetArrayItem` (`self.DialogChild`) 4) (`/Game/Prototype/Prot_ver2/W_Dialog.3-rd` (`self.Widget Dialog`))))
    (:`2`
      (bind _output_get_2 (set `/Game/Prototype/Prot_ver2/W_Dialog.DialogChar` (`self.DialogOldMan`) (`self.Widget Dialog`)))
      (set `TextBlock.Text` (`|GetArrayItem` _output_get_2) (`/Game/Prototype/Prot_ver2/W_Dialog.1-st` (`self.Widget Dialog`)))
      (bind _asbp_npc_oldman (cast `/Game/Prototype/Prot_ver2/BP_NPC_Oldman` (`self.Lockal_Something`)))
      (if (not (`/Game/Prototype/Prot_ver2/BP_NPC_Oldman.Glasses` _asbp_npc_oldman))
        (set `/Game/Prototype/Prot_ver2/BP_NPC_Oldman.Glasses` (`self.GlassesInOld`) _asbp_npc_oldman)
        (set `self.GlassesInOld` false)))
    (:`3`
      (bind _output_get_3 (set `/Game/Prototype/Prot_ver2/W_Dialog.DialogChar` (`self.DialogStandart`) (`self.Widget Dialog`)))
      (set `TextBlock.Text` (`|GetArrayItem` _output_get_3) (`/Game/Prototype/Prot_ver2/W_Dialog.1-st` (`self.Widget Dialog`)))
      (bind _asbp_npc_standart (cast `/Game/Prototype/Prot_ver2/BP_NPC_Standart` (`self.Lockal_Something`)))
      (set `/Game/Prototype/Prot_ver2/BP_NPC_Standart.Glasses` (`self.GlassesInStandart`) _asbp_npc_standart)
      (set `self.GlassesInStandart` false))
    (:`4`
      (bind _asbp_something (cast `/Game/Prototype/Prot_ver2/BP_Something` (`self.Lockal_Something`)))
      (if (`/Game/Prototype/Prot_ver2/BP_Something.IsCheck?` _asbp_something)
        (bind _output_get_4 (set `/Game/Prototype/Prot_ver2/W_Dialog.DialogChar` (`self.DialogSearch`) (`self.Widget Dialog`)))
        (set `TextBlock.Text` (`|GetArrayItem` _output_get_4) (`/Game/Prototype/Prot_ver2/W_Dialog.1-st` (`self.Widget Dialog`)))
        (set `self.Break` false)))
    (:`5`
      (if (not (`self.IsDoorCheck`))
        (bind _output_get_5 (set `/Game/Prototype/Prot_ver2/W_Dialog.DialogChar` (`self.DialogDoor`) (`self.Widget Dialog`)))
        (set `TextBlock.Text` (`|GetArrayItem` _output_get_5) (`/Game/Prototype/Prot_ver2/W_Dialog.1-st` _widget_dialog))
        (set `TextBlock.Text` (`|GetArrayItem` _output_get_5 1) (`/Game/Prototype/Prot_ver2/W_Dialog.2-nd` _widget_dialog))
        (set `TextBlock.Text` (`|GetArrayItem` _output_get_5 2) (`/Game/Prototype/Prot_ver2/W_Dialog.3-rd` _widget_dialog))))))

(event `self.ReceiveActorEndOverlap`
  (params (OtherActor :type "Actor Object Reference"))
  (bind _widget_dialog (`self.Widget Dialog`))
  (bind _widget_dialog_2 (`self.Widget Dialog`))
  (bind _pb_loot (`/Game/Prototype/Prot_ver2/W_Dialog.PB_Loot` (`self.Widget Dialog`)))
  (set `self.Lockal_Something` OtherActor)
  (switch `int` (`self.Obj`)
    (:`1`
      (cast `/Game/Prototype/Prot_ver2/BP_NPC_Child` (`self.Lockal_Something`))
      (if (`/Game/Prototype/Prot_ver2/W_Dialog.SearchStart` (`self.Widget Dialog`))
        (`KismetSystemLibrary.Delay` 0.5)
        (else
          (set `/Game/Prototype/Prot_ver2/W_Dialog.Check` false _widget_dialog_2)
          (set `/Game/Prototype/Prot_ver2/W_Dialog.CheckChild1` false _widget_dialog_2)
          (set `/Game/Prototype/Prot_ver2/W_Dialog.CheckChild2` false _widget_dialog_2))))
    (:`2`
      (cast `/Game/Prototype/Prot_ver2/BP_NPC_Oldman` (`self.Lockal_Something`)))
    (:`3`
      (cast `/Game/Prototype/Prot_ver2/BP_NPC_Standart` (`self.Lockal_Something`))
      (set `/Game/Prototype/Prot_ver2/W_Dialog.StandartCheck1` true (`self.Widget Dialog`)))
    (:`4`
      (bind _asbp_something (cast `/Game/Prototype/Prot_ver2/BP_Something` (`self.Lockal_Something`))
        (:`then`
          (if (and (<= (`ProgressBar.Percent` _pb_loot) 1.0) (`Widget.IsVisible` _pb_loot))
            (set `self.Break` true)
            (set `/Game/Prototype/Prot_ver2/BP_Something.IsCheck?` true _asbp_something)
            (set `ProgressBar.Percent` 0.0 (`/Game/Prototype/Prot_ver2/W_Dialog.PB_Loot` (`self.Widget Dialog`)))))
        (:`CastFailed`
          _)))
    (:`5`
      _))
  (set `self.Obj` 0)
  (`Widget.SetVisibility` (`/Game/Prototype/Prot_ver2/W_Dialog.Cp_Dialog` (`self.Widget Dialog`)) "Collapsed")
  (`Widget.SetVisibility` (`/Game/Prototype/Prot_ver2/W_Dialog.PB_Loot` (`self.Widget Dialog`)) "Collapsed")
  (`Widget.SetVisibility` (`/Game/Prototype/Prot_ver2/W_Dialog.1-st` (`self.Widget Dialog`)) "Collapsed")
  (`Widget.SetVisibility` (`/Game/Prototype/Prot_ver2/W_Dialog.2-nd` (`self.Widget Dialog`)) "Collapsed")
  (`Widget.SetVisibility` (`/Game/Prototype/Prot_ver2/W_Dialog.3-rd` (`self.Widget Dialog`)) "Collapsed")
  (`Widget.SetVisibility` (`/Game/Prototype/Prot_ver2/W_Dialog.Button_1` (`self.Widget Dialog`)) "Collapsed")
  (`Widget.SetVisibility` (`/Game/Prototype/Prot_ver2/W_Dialog.Button_2` (`self.Widget Dialog`)) "Collapsed")
  (`Widget.SetVisibility` (`/Game/Prototype/Prot_ver2/W_Dialog.Button_3` (`self.Widget Dialog`)) "Collapsed")
  (`Widget.SetVisibility` (`/Game/Prototype/Prot_ver2/W_Dialog.NPC` (`self.Widget Dialog`)) "Collapsed")
  (set `TextBlock.Text` "" (`/Game/Prototype/Prot_ver2/W_Dialog.1-st` _widget_dialog))
  (set `TextBlock.Text` "" (`/Game/Prototype/Prot_ver2/W_Dialog.2-nd` _widget_dialog))
  (set `TextBlock.Text` "" (`/Game/Prototype/Prot_ver2/W_Dialog.3-rd` _widget_dialog))
  (set `TextBlock.Text` "" (`/Game/Prototype/Prot_ver2/W_Dialog.NPC` _widget_dialog)))

(fn `UserConstructionScript`
  (`parent.UserConstructionScript`))