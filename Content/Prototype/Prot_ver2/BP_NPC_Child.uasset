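; Child NPC for a search quest, which registers itself and its dialog with BP_Character on overlap.
; While the dialog widget's SearchStart is set, Tick drives AI movement through five target points in reverse index order; recorded distances go unused.
; When the Glases flag is set it returns to the player, or advances QuestStatus if DefeatChild is set.
; An empty-handed search ends with a brief screen-projected speech line.
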(event `self.ReceiveBeginPlay`
  (`parent.ReceiveBeginPlay`))

(event `self.ReceiveActorBeginOverlap`
  (params (OtherActor :type "Actor Object Reference"))
  (bind _asbp_character (cast `/Game/Prototype/Prot_ver2/BP_Character` OtherActor))
  (set `/Game/Prototype/Prot_ver2/BP_Character.Something` self _asbp_character)
  (set `/Game/Prototype/Prot_ver2/BP_Character.Dialog0` (`self.Dialog0`) _asbp_character)
  (set `/Game/Prototype/Prot_ver2/BP_Character.Obj` 1 _asbp_character)
  (set `self.Character` _asbp_character))

(event `self.ReceiveTick`
  (params (DeltaSeconds :type "Float (single-precision)"))
  (bind _character (`self.Character`))
  (bind _returnvalue (`self.K2_GetActorLocation` (`self.Character`)))
  (bind _widget_dialog (`/Game/Prototype/Prot_ver2/BP_Character.Widget Dialog` (`self.Character`)))
  (`parent.ReceiveTick` DeltaSeconds)
  (`/Engine/EditorBlueprintResources/StandardMacros.IsValid` _character
    (:`Is Valid`
      (if (`/Game/Prototype/Prot_ver2/W_Dialog.SearchStart` (`/Game/Prototype/Prot_ver2/BP_Character.Widget Dialog` _character))
        (if (`self.Glases?`)
          (if (`/Game/Prototype/Prot_ver2/W_Dialog.DefeatChild` (`/Game/Prototype/Prot_ver2/BP_Character.Widget Dialog` (`self.Character`)))
            (set `/Game/Prototype/Prot_ver2/BP_Character.QuestStatus` 2 (`self.Character`))
            (else
              (`AIBlueprintHelperLibrary.SimpleMoveToLocation` (`AIBlueprintHelperLibrary.GetAIController` self) _returnvalue)
              (if (== (`self.K2_GetActorLocation`) _returnvalue :`ErrorTolerance` 20.0)
                (set `/Game/Prototype/Prot_ver2/W_Dialog.SearchEnd+` true _widget_dialog)
                (set `/Game/Prototype/Prot_ver2/W_Dialog.CheckChild1` false _widget_dialog)
                (set `/Game/Prototype/Prot_ver2/W_Dialog.CheckChild2` false _widget_dialog)
                (set `/Game/Prototype/Prot_ver2/W_Dialog.SearchStart` false _widget_dialog))))
          (else
            (`self.Search`)))))))

(event `Search`
  (bind _widget_dialog (`/Game/Prototype/Prot_ver2/BP_Character.Widget Dialog` (`self.Character`)))
  (bind _widget_dialog_2 (`/Game/Prototype/Prot_ver2/BP_Character.Widget Dialog` (`self.Character`)))
  (bind _screenlocation (`PlayerController.ProjectWorldLocationToScreen` (`GameplayStatics.GetPlayerController` 0) (`self.K2_GetActorLocation` (`self.Character`)) false))
  (bind _cp_dialog (`/Game/Prototype/Prot_ver2/W_Dialog.Cp_Dialog` _widget_dialog_2))
  (bind _returnvalue (`self.K2_GetActorLocation` (`|GetArrayItem` (`self.TargetPoints`) (- (`self.IntDot2`) 1))))
  (if (== (`self.IntDot`) 5) :!label _label
    (switch `int` (`self.IntDot2`) :!label _label_2
      (:`0`
        (`AIBlueprintHelperLibrary.SimpleMoveToLocation` (`AIBlueprintHelperLibrary.GetAIController` self) (`self.K2_GetActorLocation` (`self.Character`)))
        (set `/Game/Prototype/Prot_ver2/W_Dialog.SearchEnd-` true _widget_dialog_2)
        (set `/Game/Prototype/Prot_ver2/W_Dialog.CheckChild1` false _widget_dialog_2)
        (set `/Game/Prototype/Prot_ver2/W_Dialog.CheckChild2` false _widget_dialog_2)
        (set `/Game/Prototype/Prot_ver2/W_Dialog.SearchStart` false _widget_dialog_2)
        (`Widget.SetRenderTranslation` (`/Game/Prototype/Prot_ver2/W_Dialog.Cp_Dialog` (`/Game/Prototype/Prot_ver2/BP_Character.Widget Dialog` (`self.Character`))) (`KismetMathLibrary.MakeVector2D` (`KismetMathLibrary.BreakVector2D` _screenlocation) (- (`.Y` (`KismetMathLibrary.BreakVector2D` _screenlocation)) 150.0)))
        (set `TextBlock.Text` (`|GetArrayItem` (`/Game/Prototype/Prot_ver2/BP_Character.DialogChild` (`self.Character`)) 3) (`/Game/Prototype/Prot_ver2/W_Dialog.1-st` _widget_dialog_2))
        (`Widget.SetVisibility` _cp_dialog "Visible")
        (`Widget.SetVisibility` (`/Game/Prototype/Prot_ver2/W_Dialog.1-st` _widget_dialog_2) "Visible")
        (`KismetSystemLibrary.Delay` 1.0)
        (`Widget.SetVisibility` _cp_dialog "Collapsed")
        (`Widget.SetVisibility` (`/Game/Prototype/Prot_ver2/W_Dialog.1-st` _widget_dialog_2) "Collapsed"))
      (:`1`
        (`AIBlueprintHelperLibrary.SimpleMoveToLocation` (`AIBlueprintHelperLibrary.GetAIController` self) _returnvalue :!label _label_3)
        (if (== (`self.K2_GetActorLocation` self) _returnvalue :`ErrorTolerance` 90.0)
          (`KismetSystemLibrary.Delay` 2.0)
          (set `self.IntDot2` (- (`self.IntDot2`) 1))
          (if (`self.Glases?`)
            (`AIBlueprintHelperLibrary.SimpleMoveToLocation` (`AIBlueprintHelperLibrary.GetAIController` self) (`self.K2_GetActorLocation` (`self.Character`)))
            (set `/Game/Prototype/Prot_ver2/W_Dialog.SearchEnd+` true _widget_dialog)
            (set `/Game/Prototype/Prot_ver2/W_Dialog.SearchStart` false _widget_dialog)
            (else
              (goto _label_2)))))
      (:`2`
        (goto _label_3))
      (:`3`
        (goto _label_3))
      (:`4`
        (goto _label_3))
      (:`5`
        (goto _label_3)))
    (else
      (`KismetArrayLibrary.Array_Add` (`self.Distance`) (`self.GetDistanceTo` (`|GetArrayItem` (`self.TargetPoints`) (`self.IntDot`)) self))
      (set `self.IntDot` (+ (`self.IntDot`) 1))
      (set `self.IntDot2` (`self.IntDot`))
      (goto _label))))

(fn `UserConstructionScript`
  (`parent.UserConstructionScript`))