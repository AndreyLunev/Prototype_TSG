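; BP_Something is a prototype overlap-triggered actor that registers itself with the player character or passes glasses to child NPCs.
; On overlap, a BP_Character receives a reference to this actor and has its Obj index set to 4.
; A BP_NPC_Child with an unset Glases value waits through a short delay, then receives this actor's Glasses value if still overlapping.
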(event `self.ReceiveBeginPlay`)

(event `self.ReceiveActorBeginOverlap`
  (params (OtherActor :type "Actor Object Reference"))
  (bind _asbp_character (cast `/Game/Prototype/Prot_ver2/BP_Character` OtherActor)
    (:`then`
      (set `/Game/Prototype/Prot_ver2/BP_Character.Something` self _asbp_character)
      (set `/Game/Prototype/Prot_ver2/BP_Character.Obj` 4 _asbp_character))
    (:`CastFailed`
      (bind _asbp_npc_child (cast `/Game/Prototype/Prot_ver2/BP_NPC_Child` OtherActor))
      (if (not (`/Game/Prototype/Prot_ver2/BP_NPC_Child.Glases?` _asbp_npc_child))
        (`KismetSystemLibrary.Delay` 1.7)
        (if (`self.IsOverlappingActor` _asbp_npc_child self)
          (set `/Game/Prototype/Prot_ver2/BP_NPC_Child.Glases?` (`self.Glasses`) _asbp_npc_child))))))

(fn `UserConstructionScript`)