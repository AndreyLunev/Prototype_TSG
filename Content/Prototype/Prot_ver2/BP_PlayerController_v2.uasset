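; Prototype player controller that provides click-and-hold movement to the point under the cursor.
; The Move input opens a gate on press and closes it on release.
; While the gate is open, each Tick traces under the cursor on the Visibility channel and sends the hit location to SimpleMoveToLocation.
; BeginPlay casts the player character to BP_Character but does nothing with the result.
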(event `self.ReceiveBeginPlay`
  (cast `/Game/Prototype/Prot_ver2/BP_Character` (`GameplayStatics.GetPlayerCharacter` 0)))

(event `self.ReceiveTick`
  (params (DeltaSeconds :type "Float (single-precision)"))
  (`/Engine/EditorBlueprintResources/StandardMacros.Gate` true :!label _label
    (:`Exit`
      (`self.Move to Hit Location` (`self.GetHitResultUnderCursorByChannel` "TraceTypeQuery1")))))

(event `InputAction|Move`
  (params (Key :type "Key Structure"))
  (:`Pressed`
    (goto _label :!via `Open`))
  (:`Released`
    (goto _label :!via `Close`)))

(fn `Move to Hit Location`
  (params (Hit :type "HitResult Structure"))
  (locals (MinDistance :type "Float (double-precision)"))
  (`AIBlueprintHelperLibrary.SimpleMoveToLocation` self (`.Location` (`GameplayStatics.BreakHitResult` Hit))))

(fn `UserConstructionScript`)