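; BP_Enter is a prototype actor that turns parts of itself see-through while a BP_Character overlaps it, apparently as an enterable structure.
; Begin overlap swaps the first material slot of Cube1, Plane and Plane1 to M_Transparent, and end overlap sets it to M_Base.
; Both events cast the other actor to BP_Character, so other actors do not trigger the swap.
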(event `self.ReceiveActorBeginOverlap`
  (params (OtherActor :type "Actor Object Reference"))
  (cast `/Game/Prototype/Prot_ver2/BP_Character` OtherActor)
  (`PrimitiveComponent.SetMaterial` (`self.Cube1`) 0 "/Game/Prototype/Prot_ver2/M_Transparent.M_Transparent")
  (`PrimitiveComponent.SetMaterial` (`self.Plane`) 0 "/Game/Prototype/Prot_ver2/M_Transparent.M_Transparent")
  (`PrimitiveComponent.SetMaterial` (`self.Plane1`) 0 "/Game/Prototype/Prot_ver2/M_Transparent.M_Transparent"))

(event `self.ReceiveActorEndOverlap`
  (params (OtherActor :type "Actor Object Reference"))
  (cast `/Game/Prototype/Prot_ver2/BP_Character` OtherActor)
  (`PrimitiveComponent.SetMaterial` (`self.Cube1`) 0 "/Game/Prototype/Prot_ver2/M_Base.M_Base")
  (`PrimitiveComponent.SetMaterial` (`self.Plane`) 0 "/Game/Prototype/Prot_ver2/M_Base.M_Base")
  (`PrimitiveComponent.SetMaterial` (`self.Plane1`) 0 "/Game/Prototype/Prot_ver2/M_Base.M_Base"))

(fn `UserConstructionScript`)