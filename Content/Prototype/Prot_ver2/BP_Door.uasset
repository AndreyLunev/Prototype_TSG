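; Prototype door that hands the overlapping BP_Character a dialog and can spawn an NPC behind it.
; On overlap it registers itself as the character's current object and picks the dialog from IsSomebody, IsQuest and Who.
; Tick polls the dialog widget's WantToSpawn flag, then once shifts the character along world X.
; Depending on Who, it spawns a standard or old-man NPC, clears the flag and destroys its Box.
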(event `self.ReceiveBeginPlay`)

(event `self.ReceiveActorBeginOverlap`
  (params (OtherActor :type "Actor Object Reference"))
  (bind _asbp_character (cast `/Game/Prototype/Prot_ver2/BP_Character` OtherActor))
  (set `self.As BP Character` _asbp_character)
  (set `/Game/Prototype/Prot_ver2/BP_Character.Something` self _asbp_character)
  (set `/Game/Prototype/Prot_ver2/BP_Character.IsDoorCheck` false _asbp_character)
  (set `/Game/Prototype/Prot_ver2/BP_Character.Obj` 5 _asbp_character)
  (if (`self.Is_Somebody?`)
    (if (`self.Is_Quest?`)
      (set `/Game/Prototype/Prot_ver2/BP_Character.Dialog0` (`self.Dialog_Quest`) (`self.As BP Character`))
      (else
        (switch `int` (`self.Who?`)
          (:`1`
            (set `/Game/Prototype/Prot_ver2/BP_Character.Dialog0` (`self.Dialog_1`) (`self.As BP Character`)))
          (:`2`
            (set `/Game/Prototype/Prot_ver2/BP_Character.Dialog0` (`self.Dialog_2`) (`self.As BP Character`))))))
    (else
      (set `/Game/Prototype/Prot_ver2/BP_Character.Dialog0` (`self.Dialog_0`) _asbp_character))))

(event `self.ReceiveTick`
  (params (DeltaSeconds :type "Float (single-precision)"))
  (bind (_returnvalue_x _returnvalue_y _returnvalue_z) (`KismetMathLibrary.BreakVector` (`self.K2_GetActorLocation`)))
  (bind (_returnvalue_x_2 _returnvalue_y_2 _returnvalue_z_2) (`KismetMathLibrary.BreakVector` (`self.K2_GetActorLocation`)))
  (bind _as_bp_character (`self.As BP Character`))
  (bind _as_bp_character_2 (`self.As BP Character`))
  (bind (_returnvalue_x_3 _returnvalue_y_3 _returnvalue_z_3) (`KismetMathLibrary.BreakVector` (`self.K2_GetActorLocation` _as_bp_character_2)))
  (`/Engine/EditorBlueprintResources/StandardMacros.IsValid` _as_bp_character
    (:`Is Valid`
      (if (`/Game/Prototype/Prot_ver2/W_Dialog.WantToSpawn` (`/Game/Prototype/Prot_ver2/BP_Character.Widget Dialog` _as_bp_character))
        (`/Engine/EditorBlueprintResources/StandardMacros.DoOnce` false
          (:`Completed`
            (`self.K2_SetActorLocation` _as_bp_character_2 (`KismetMathLibrary.MakeVector` (+ _returnvalue_x_3 180.0) _returnvalue_y_3 _returnvalue_z_3) false false)
            (switch `int` (`self.Who?`)
              (:`2`
                (`|SpawnActorFromClass` "/Game/Prototype/Prot_ver2/BP_NPC_Standart.BP_NPC_Standart_C" (`KismetMathLibrary.MakeTransform` (`KismetMathLibrary.MakeVector` (+ _returnvalue_x 120.0) _returnvalue_y (- _returnvalue_z 120.0))) "AlwaysSpawn" "OverrideRootScale" null null))
              (:`3`
                (`|SpawnActorFromClass` "/Game/Prototype/Prot_ver2/BP_NPC_Oldman.BP_NPC_Oldman_C" (`KismetMathLibrary.MakeTransform` (`KismetMathLibrary.MakeVector` (+ _returnvalue_x_2 120.0) _returnvalue_y_2 (- _returnvalue_z_2 120.0))) "AlwaysSpawn" "OverrideRootScale" null null)))
            (set `/Game/Prototype/Prot_ver2/W_Dialog.WantToSpawn` false (`/Game/Prototype/Prot_ver2/BP_Character.Widget Dialog` (`self.As BP Character`)))
            (`ActorComponent.K2_DestroyComponent` (`self.Box`))))))))

(fn `UserConstructionScript`)