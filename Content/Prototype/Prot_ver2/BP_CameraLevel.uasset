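; BP_CameraLevel is a prototype overlap volume that shifts the player's camera height while BP_Character is inside it.
; On begin overlap it casts to BP_Character and raises that character's Camera actor by a fixed Z offset.
; On end overlap it lowers the camera by the same amount, using instant relative location changes with no interpolation.
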(event `self.ReceiveActorBeginOverlap`
  (params (OtherActor :type "Actor Object Reference"))
  (bind _asbp_character (cast `/Game/Prototype/Prot_ver2/BP_Character` OtherActor))
  (bind _camera (`/Game/Prototype/Prot_ver2/C++Blueprints/Character.Camera` _asbp_character))
  (bind (_returnvalue_x _returnvalue_y _returnvalue_z) (`KismetMathLibrary.BreakVector` (`self.K2_GetActorLocation` _camera)))
  (`self.K2_SetActorLocation` _camera (`KismetMathLibrary.MakeVector` _returnvalue_x _returnvalue_y (+ _returnvalue_z 250.0)) false false))

(event `self.ReceiveActorEndOverlap`
  (params (OtherActor :type "Actor Object Reference"))
  (bind _asbp_character (cast `/Game/Prototype/Prot_ver2/BP_Character` OtherActor))
  (bind _camera (`/Game/Prototype/Prot_ver2/C++Blueprints/Character.Camera` _asbp_character))
  (bind (_returnvalue_x _returnvalue_y _returnvalue_z) (`KismetMathLibrary.BreakVector` (`self.K2_GetActorLocation` _camera)))
  (`self.K2_SetActorLocation` _camera (`KismetMathLibrary.MakeVector` _returnvalue_x _returnvalue_y (+ _returnvalue_z -250.0)) false false))

(fn `UserConstructionScript`)